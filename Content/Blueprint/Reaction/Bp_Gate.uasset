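; Gate actor that moves along a spline when its Reaction event fires, likely triggered by another object in the level.
; Reaction plays the Move timeline, whose Distance track is scaled by the spline's length.
; Each update samples the spline at that distance in world space and sets the Gate component's location there, without sweeping.
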(event `self.Reaction`
  (bind (_direction _distance) (`Timeline|Move`)
    (:`Update`
      (`SceneComponent.K2_SetWorldLocation` (`self.Gate`) (`SplineComponent.GetLocationAtDistanceAlongSpline` (`self.Spline`) (* _distance (`SplineComponent.GetSplineLength` (`self.Spline`))) "World") false false))))

(fn `UserConstructionScript`
  (`parent.UserConstructionScript`))