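; A movable platform actor that travels along a spline and can be started or halted through its Reaction event.
; The MovePlatform timeline scales its Distance track by spline length to set the platform's world location, plus roll and yaw with pitch held at zero.
; It plays on BeginPlay if Start is set, and Reaction toggles that flag to play or stop it.
; The construction script pre-aligns the platform to the spline's start rotation.
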(event `self.ReceiveBeginPlay`
  (bind _spline (`self.Spline`))
  (bind _platform (`self.Platform`))
  (`parent.ReceiveBeginPlay`)
  (if (`self.Start`)
    (bind (_direction _distance) (`Timeline|MovePlatform` :!label _label)
      (:`Update`
        (bind _returnvalue (* _distance (`SplineComponent.GetSplineLength` (`self.Spline`))))
        (`SceneComponent.K2_SetWorldLocation` _platform (`SplineComponent.GetLocationAtDistanceAlongSpline` _spline _returnvalue "World") false false)
        (bind (_returnvalue_roll _returnvalue_pitch _returnvalue_yaw) (`KismetMathLibrary.BreakRotator` (`SplineComponent.GetRotationAtDistanceAlongSpline` _spline _returnvalue "Local")))
        (`SceneComponent.K2_SetWorldRotation` _platform (`KismetMathLibrary.MakeRotator` _returnvalue_roll 0.0 _returnvalue_yaw) false false)))))

(event `self.Reaction`
  (if (`self.Start`)
    (set `self.Start` false)
    (goto _label :!via `Stop`)
    (else
      (set `self.Start` true)
      (goto _label))))

(fn `UserConstructionScript`
  (bind (_returnvalue_roll _returnvalue_pitch _returnvalue_yaw) (`KismetMathLibrary.BreakRotator` (`SplineComponent.GetRotationAtDistanceAlongSpline` (`self.Spline`) 0.0 "Local")))
  (`parent.UserConstructionScript`)
  ;[1 1 1] Set platform rotation, depending of spline direction
  (`SceneComponent.K2_SetWorldRotation` (`self.Platform`) (`KismetMathLibrary.MakeRotator` _returnvalue_roll 0.0 _returnvalue_yaw) false false))