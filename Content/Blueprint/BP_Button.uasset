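; BP_Button is an interactable button that animates, plays a sound and triggers a Reaction on ActorReaction when pressed.
; A Sphere overlap enables input and opens a gate for BP_Player, so Interact works only until the player leaves.
; The Button Animation graph lerps the button between its starting transform and a slightly lowered one, using one timeline in and another reversed out.
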(event `self.ReceiveBeginPlay`
  (bind (_returnvalue_location _returnvalue_rotation _returnvalue_scale) (`KismetMathLibrary.BreakTransform` (`SceneComponent.GetRelativeTransform` (`self.Button`))))
  ;[1 1 1] Set Button Out and In positions
  (set `self.OutTransfom` (`KismetMathLibrary.MakeTransform` _returnvalue_location _returnvalue_rotation _returnvalue_scale))
  (set `self.InTransform` (`KismetMathLibrary.MakeTransform` (- _returnvalue_location (0.0 0.0 5.0)) _returnvalue_rotation _returnvalue_scale)))

(event `InputAction|Interact`
  (params (Key :type "Key Structure"))
  (:`Pressed`
    (`/Engine/EditorBlueprintResources/StandardMacros.Gate` true :!label _label
      (:`Exit`
        (`GameplayStatics.PlaySoundAtLocation` "/Game/Sound/S_Button.S_Button" (`SceneComponent.K2_GetComponentLocation` (`self.Button`)) (struct) 1.0 1.0 0.0 null null null)
        (bind (_direction _track) (`Timeline|Button In` :!via `PlayFromStart`)
          (:`Update`
            (`SceneComponent.K2_SetRelativeTransform` (`self.Button`) (`KismetMathLibrary.TLerp` (`self.OutTransfom`) (`self.InTransform`) _track) false false))
          (:`Finished`
            (bind (_direction_2 _button_in) (`Timeline|Button Out` :!via `ReverseFromEnd`)
              (:`Update`
                (`SceneComponent.K2_SetRelativeTransform` (`self.Button`) (`KismetMathLibrary.TLerp` (`self.OutTransfom`) (`self.InTransform`) _button_in) false false))
              (:`Finished`
                (`/Game/Blueprint/Reaction/BP_Reaction.Reaction` (`self.ActorReaction`))))))))))

(event `self.Sphere.OnComponentBeginOverlap`
  (params (OverlappedComponent :type "PrimitiveComponent Object Reference") (OtherActor :type "Actor Object Reference") (OtherComp :type "PrimitiveComponent Object Reference") (OtherBodyIndex :type Integer) (bFromSweep :type Boolean) (SweepResult :type "HitResult Structure (by ref)"))
  (`self.EnableInput` (`GameplayStatics.GetPlayerController` 0))
  (cast `/Game/Blueprint/BP_Player` OtherActor)
  (goto _label :!via `Open`))

(event `self.Sphere.OnComponentEndOverlap`
  (params (OverlappedComponent :type "PrimitiveComponent Object Reference") (OtherActor :type "Actor Object Reference") (OtherComp :type "PrimitiveComponent Object Reference") (OtherBodyIndex :type Integer))
  (cast `/Game/Blueprint/BP_Player` OtherActor)
  (goto _label :!via `Close`))

(fn `UserConstructionScript`)