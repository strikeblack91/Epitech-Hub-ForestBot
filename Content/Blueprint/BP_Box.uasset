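; BP_Box is a physics box actor that returns to its starting position after falling out of the level.
; BeginPlay stores the world location of the Box component.
; Each Tick checks whether its height has dropped below a fixed Z threshold, then moves it back to the stored location and zeroes its linear velocity.
; Rotation and angular velocity are left unchanged.
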(event `self.ReceiveBeginPlay`
  (set `self.Location` (`SceneComponent.K2_GetComponentLocation` (`self.Box`))))

(event `self.ReceiveTick`
  (params (DeltaSeconds :type "Float (single-precision)"))
  (bind (_returnvalue_x _returnvalue_y _returnvalue_z) (`KismetMathLibrary.BreakVector` (`SceneComponent.K2_GetComponentLocation` (`self.Box`))))
  (if (< _returnvalue_z -500.0)
    (`SceneComponent.K2_SetWorldLocation` (`self.Box`) (`self.Location`) false false)
    (`PrimitiveComponent.SetAllPhysicsLinearVelocity` (`self.Box`) (0.0 0.0 0.0) false)))

(fn `UserConstructionScript`)