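; BP_Platform is a trigger platform that notifies a referenced actor when something enters or leaves its Box volume.
; Both begin and end overlap call the same Reaction on that actor, with no filter on the overlapping object.
; BeginPlay caches the Body's resting transform and a slightly lowered "in" transform, though nothing here moves the Body.
; Disconnected leftover nodes refer to an older Button and ActorReaction setup.
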(event `self.ReceiveBeginPlay`
  (bind (_returnvalue_location _returnvalue_rotation _returnvalue_scale) (`KismetMathLibrary.BreakTransform` (`SceneComponent.GetRelativeTransform` (`self.Body`))))
  (set `self.OutTransform` (`KismetMathLibrary.MakeTransform` _returnvalue_location _returnvalue_rotation _returnvalue_scale))
  (set `self.InTransform` (`KismetMathLibrary.MakeTransform` (- _returnvalue_location (0.0 0.0 5.0)) _returnvalue_rotation _returnvalue_scale)))

(event `self.Box.OnComponentBeginOverlap`
  (params (OverlappedComponent :type "PrimitiveComponent Object Reference") (OtherActor :type "Actor Object Reference") (OtherComp :type "PrimitiveComponent Object Reference") (OtherBodyIndex :type Integer) (bFromSweep :type Boolean) (SweepResult :type "HitResult Structure (by ref)"))
  (`/Game/Blueprint/Reaction/BP_Reaction.Reaction` (`self.Actor`) :!label _label))

(event `self.Box.OnComponentEndOverlap`
  (params (OverlappedComponent :type "PrimitiveComponent Object Reference") (OtherActor :type "Actor Object Reference") (OtherComp :type "PrimitiveComponent Object Reference") (OtherBodyIndex :type Integer))
  (goto _label))

(fn `UserConstructionScript`)