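; Checkpoint actor that spins continuously and saves a respawn position on the player who touches it.
; On mesh overlap with BP_Player, it passes the mesh's world location, raised by a height offset, to the player's SetCheckpoint.
; An equality check against the player's stored position skips repeat activations, so the effect and sound only play when the checkpoint changes.
; The spin is a fixed per-tick rotation, so its speed depends on frame rate.
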(event `self.ReceiveTick`
  (params (DeltaSeconds :type "Float (single-precision)"))
  (`self.K2_AddActorLocalRotation` self (struct :`Yaw` 1.0) false false))

(event `self.StaticMesh.OnComponentBeginOverlap`
  (params (OverlappedComponent :type "PrimitiveComponent Object Reference") (OtherActor :type "Actor Object Reference") (OtherComp :type "PrimitiveComponent Object Reference") (OtherBodyIndex :type Integer) (bFromSweep :type Boolean) (SweepResult :type "HitResult Structure (by ref)"))
  (bind (_returnvalue_x _returnvalue_y _returnvalue_z) (`KismetMathLibrary.BreakVector` (`SceneComponent.K2_GetComponentLocation` (`self.StaticMesh`))))
  (bind (_returnvalue_x_2 _returnvalue_y_2 _returnvalue_z_2) (`KismetMathLibrary.BreakVector` (`SceneComponent.K2_GetComponentLocation` (`self.StaticMesh`))))
  (bind _asbp_player (cast `/Game/Blueprint/BP_Player` OtherActor))
  (if (`KismetMathLibrary.NotEqualExactly_VectorVector` (`/Game/Blueprint/BP_Player.CheckpointPosition` _asbp_player) (`KismetMathLibrary.MakeVector` _returnvalue_x _returnvalue_y (+ _returnvalue_z (`self.Offset`))))
    (`/Game/Blueprint/BP_Player.SetCheckpoint` _asbp_player (`KismetMathLibrary.MakeVector` _returnvalue_x_2 _returnvalue_y_2 (+ _returnvalue_z_2 (`self.Offset`))))
    (`ActorComponent.Activate` (`self.Effect`) false)
    (`GameplayStatics.PlaySoundAtLocation` "/Game/Sound/S_Checkpoint.S_Checkpoint" (`SceneComponent.K2_GetComponentLocation` (`self.StaticMesh`)) (struct) 1.0 1.0 0.0 null null null)))

(fn `UserConstructionScript`)