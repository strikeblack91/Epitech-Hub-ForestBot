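; BP_Canon is a cannon actor that repeatedly fires physics projectiles on a fixed looping timer.
; BeginPlay starts the timer, optionally after a random delay between DelayMin and DelayMax.
; Fire spawns a half-scale BP_Projectile at the Cylinder, activates the particle effect, overrides the projectile's mass with Weight, and launches it along the Direction component's forward vector as a velocity-change impulse scaled by Strength.
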(event `self.ReceiveBeginPlay`
  (if (`self.IsDelay`)
    (`KismetSystemLibrary.Delay` (`KismetMathLibrary.RandomFloatInRange` (`self.DelayMin`) (`self.DelayMax`)))
    (`KismetSystemLibrary.K2_SetTimer` null "Fire" 2.0 true)
    (else
      (`KismetSystemLibrary.K2_SetTimer` null "Fire" 2.0 true))))

(fn `Fire`
  (bind (_returnvalue_location _returnvalue_rotation) (`KismetMathLibrary.BreakTransform` (`SceneComponent.K2_GetComponentToWorld` (`self.Cylinder`))))
  (bind _returnvalue (`|SpawnActorFromClass` "/Game/Blueprint/BP_Projectile.BP_Projectile_C" (`KismetMathLibrary.MakeTransform` _returnvalue_location _returnvalue_rotation (0.5 0.5 0.5)) "Undefined" "OverrideRootScale" null null))
  (`ActorComponent.Activate` (`self.ParticleSystem`) false)
  (bind _sphere (`/Game/Blueprint/BP_Projectile.Sphere` _returnvalue))
  (`PrimitiveComponent.SetMassOverrideInKg` _sphere "None" (`self.Weight`) true)
  (`PrimitiveComponent.AddImpulse` _sphere (* (`SceneComponent.GetForwardVector` (`self.Direction`)) (`self.Strength`)) "None" true))

(fn `UserConstructionScript`)