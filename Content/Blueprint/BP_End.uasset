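; BP_End is a spinning level-exit actor that ends a level when the player touches it.
; It rotates a little every tick, and its mesh overlap responds only to BP_Player.
; On overlap it loads the LevelSaved save slot, calls UnlockLevel with the configured index minus one, then opens the level named by LevelName.
; No save call follows the unlock here.
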(event `self.ReceiveTick`
  (params (DeltaSeconds :type "Float (single-precision)"))
  (`self.K2_AddActorLocalRotation` self (struct :`Yaw` 1.0) false false))

(event `self.StaticMesh.OnComponentBeginOverlap`
  (params (OverlappedComponent :type "PrimitiveComponent Object Reference") (OtherActor :type "Actor Object Reference") (OtherComp :type "PrimitiveComponent Object Reference") (OtherBodyIndex :type Integer) (bFromSweep :type Boolean) (SweepResult :type "HitResult Structure (by ref)"))
  (cast `/Game/Blueprint/BP_Player` OtherActor)
  (bind _returnvalue (`GameplayStatics.LoadGameFromSlot` "LevelSaved"))
  (bind _ass_level_saved (cast `/Game/Blueprint/S_LevelSaved` _returnvalue))
  (`/Game/Blueprint/S_LevelSaved.UnlockLevel` _ass_level_saved (- (`self.IndexLevelUnlock`) 1))
  (`GameplayStatics.OpenLevel` (`self.LevelName`)))

(fn `UserConstructionScript`)